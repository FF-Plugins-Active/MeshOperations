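; BP_Template_MeshOperations is a template Blueprint that gathers mesh and hierarchy utility calls, none of which are wired to execute.
; Unconnected nodes cover renaming via ACRename, transform recording, empty-root cleanup, scene, static and procedural mesh component creation, vertex access, pivot moves and height or center optimization.
; A stub custom event serves as the delegate for recursive pivot centering, and the construction script is empty.
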(event `CustomEvent_0`
  (params (IsSuccessfull :type Boolean))
  ;[1 1 1] Static Functions
)

(fn `UserConstructionScript`)